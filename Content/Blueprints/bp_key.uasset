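; A collectible key pickup actor that adds to the player's key count.
; When its Box collider is overlapped by a BP_ThirdPersonCharacter, it increments that character's KeyCount and destroys itself.
; On-screen debug prints report the key's presence at BeginPlay, each pickup with the new count, and a failed cast for other overlapping actors.
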(event OnComponentBeginOverlap(Box)
  (params (OverlappedComponent :type Primitive%20Component%20Object%20Reference) (OtherActor :type Actor%20Object%20Reference) (OtherComp :type Primitive%20Component%20Object%20Reference) (OtherBodyIndex :type Integer) (bFromSweep :type Boolean) (SweepResult :type Hit%20Result%20Structure%20%28by%20ref%29))
  (bind _asbp_third_person_character (Utilities|Casting|CastToBP_ThirdPersonCharacter OtherActor)
    (:then
      (Development|PrintString "A Player has ontained the key!" true true "(R=0.000000,G=0.660000,B=1.000000,A=1.000000)" 5.0)
      (Variables|/Game/ThirdPerson/Blueprints/BP_ThirdPersonCharacter.BP_ThirdPersonCharacter_C|SetkeyCount _asbp_third_person_character (+ (Variables|/Game/ThirdPerson/Blueprints/BP_ThirdPersonCharacter.BP_ThirdPersonCharacter_C|GetkeyCount _asbp_third_person_character) 1))
      (Development|PrintString (Utilities|String|Append "The Player has " (Utilities|String|ToString(Integer) (Variables|/Game/ThirdPerson/Blueprints/BP_ThirdPersonCharacter.BP_ThirdPersonCharacter_C|GetkeyCount _asbp_third_person_character)) " key(s)."))
      (Actor|DestroyActor))
    (:CastFailed
      (Development|PrintString "Key Player Cast Failed :(" true true "(R=1.000000,G=0.229378,B=0.349274,A=1.000000)" 3.0))))

(event EventBeginPlay
  (Development|PrintString "A Key exists in the scene" true true "(R=0.398619,G=1.000000,B=0.137867,A=1.000000)"))

(fn ConstructionScript)