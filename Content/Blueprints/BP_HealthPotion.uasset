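; Health potion actor that a BP_ThirdPersonCharacter can pick up, drop and use.
; Overlapping PickupTrigger passes it to the character's TryToPickup; Pickup snaps it to the hand_r socket, and Drop detaches it and enables Cone physics and collision.
; PrimaryAction only prints a heal message and destroys the actor, with no health change.
; The node clearing the character's HeldItem is unconnected, so it never runs.
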(event OnComponentBeginOverlap(pickuptrigger)
  (params (OverlappedComponent :type Primitive%20Component%20Object%20Reference) (OtherActor :type Actor%20Object%20Reference) (OtherComp :type Primitive%20Component%20Object%20Reference) (OtherBodyIndex :type Integer) (bFromSweep :type Boolean) (SweepResult :type Hit%20Result%20Structure%20%28by%20ref%29))
  (bind _asbp_third_person_character (Utilities|Casting|CastToBP_ThirdPersonCharacter OtherActor))
  (Default|TrytoPickup _asbp_third_person_character self))

(event EventBeginPlay)

(event Collision|EventActorBeginOverlap
  (params (OtherActor :type Actor%20Object%20Reference)))

(event EventTick
  (params (DeltaSeconds :type Float%20%28single-precision%29)))

(event EventPickup
  (params (ParentMesh :type Skeletal%20Mesh%20Component%20Object%20Reference))
  (Transformation|AttachComponentToComponent (Variables|Default|GetDefaultSceneRoot) ParentMesh "hand_r" "SnapToTarget" "KeepRelative" "KeepRelative" true))

(event EventDrop
  (Transformation|DetachFromComponent (Variables|Default|GetDefaultSceneRoot) "KeepRelative" "KeepRelative" "KeepRelative" true)
  (Physics|SetSimulatePhysics (Variables|Default|GetCone) true)
  (Collision|SetCollisionEnabled (Variables|Default|GetCone) "QueryAndPhysics"))

(event EventPrimaryAction
  (params (ref_thidPersonCharacter :type BP%20Third%20Person%20Character%20Object%20Reference))
  (Development|PrintString "+10 hp" true true "(R=1.000000,G=0.000000,B=0.269310,A=1.000000)")
  (Actor|DestroyActor))

(fn ConstructionScript)