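; Falling platform that drops shortly after the third-person character enters its trigger box, then returns to its starting pose.
; Delays chain Activate, Drop and Reset, switching physics on for the fall and swapping the cube's material per state.
; Reset uses a timeline to lerp the cube back to the transform saved at BeginPlay.
; Each overlap sets Ready before Activate checks it, so that flag does not block re-triggering.
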(event OnComponentBeginOverlap(Box)
  (params (OverlappedComponent :type Primitive%20Component%20Object%20Reference) (OtherActor :type Actor%20Object%20Reference) (OtherComp :type Primitive%20Component%20Object%20Reference) (OtherBodyIndex :type Integer) (bFromSweep :type Boolean) (SweepResult :type Hit%20Result%20Structure%20%28by%20ref%29))
  (Utilities|Casting|CastToBP_ThirdPersonCharacter OtherActor)
  (Variables|Default|SetReady true)
  (CallFunction|Activate))

(event Custom|Activate
  (if (Variables|Default|GetReady)
    (Variables|Default|SetReady false)
    (Rendering|Material|SetMaterial (Variables|Default|GetCube) 0 "/Game/Materials/MI_PlatformActivated.MI_PlatformActivated")
    (Utilities|FlowControl|Delay 1.0)
    (CallFunction|Drop)))

(event Custom|Drop
  (Physics|SetSimulatePhysics (Variables|Default|GetCube) true)
  (Rendering|Material|SetMaterial (Variables|Default|GetCube) 0 "/Game/Materials/MI_PlatformFalling.MI_PlatformFalling")
  (Utilities|FlowControl|Delay 3.0)
  (CallFunction|Reset))

(event Custom|Reset
  (Variables|Default|SetResetTransform (Transformation|GetWorldTransform (Variables|Default|GetCube)))
  (Physics|SetSimulatePhysics (Variables|Default|GetCube) false)
  (Rendering|Material|SetMaterial (Variables|Default|GetCube) 0 "/Game/Materials/MI_PlatformResetting.MI_PlatformResetting")
  (bind _newtrack_0 (Timeline|Go%20Back%20To%20Start PlayFromStart)
    (:Update
      (Transformation|SetWorldLocationAndRotation (Variables|Default|GetCube) (.location (Math|Transform|Lerp(Transform) (Variables|Default|GetResetTransform) (Variables|Default|GetStartingTransform) _newtrack_0)) (.rotation (Math|Transform|Lerp(Transform) (Variables|Default|GetResetTransform) (Variables|Default|GetStartingTransform) _newtrack_0)) false false))
    (:Finished
      (Variables|Default|SetReady true)
      (Rendering|Material|SetMaterial (Variables|Default|GetCube) 0 "/Game/Materials/MI_PlatformFine.MI_PlatformFine"))))

(event EventBeginPlay
  (Variables|Default|SetStartingTransform (Transformation|GetWorldTransform (Variables|Default|GetCube))))

(event Collision|EventActorBeginOverlap
  (params (OtherActor :type Actor%20Object%20Reference)))

(event EventTick
  (params (DeltaSeconds :type Float%20%28single-precision%29)))

(fn ConstructionScript)