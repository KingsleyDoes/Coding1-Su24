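; Practice actor for loops and arrays that prints debug messages and recolors Bp_key actors.
; On BeginPlay it enables input, gathers the keys and starts ChangeKeyColor, which re-calls itself after a short Delay to tint a key through a dynamic material.
; Its reversed color-length check reshuffles both arrays on virtually every pass.
; Inputs trigger a while loop and name-array printouts; the game-loop and recursion events are empty, their logic disconnected.
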(event Custom|Simple%20Game%20Loop)

(event Custom|recursivve%20loop)

(event Custom|FirstArray%20Test
  (bind _array (Utilities|Array|MakeArray "Laken" "Luke" "Ryu" "Cass" "Latisha" "Gail"))
  (Development|PrintString (Utilities|String|Append "Our array of names has " (Utilities|String|ToString(Integer) (Utilities|Array|Length _array)) " names in  it."))
  (Development|PrintString (Utilities|String|Append "The first name in the array is " (Utilities|Array|Get(acopy) _array))))

(event Custom|ListAllNames
  (for (_array_element _array_index) (Utilities|Array|MakeArray "Laken" "Luke" "Ryu" "Cass" "Latisha" "Gail")
    (Development|PrintString (Utilities|String|Append (Utilities|String|ToString(Integer) (+ _array_index 1)) ". " _array_element) true true "(R=0.893472,G=1.000000,B=0.000000,A=1.000000)")))

(event Custom|Change%20Key%20color
  (if (or (>= (Utilities|Array|Length (Variables|Default|GetColor)) (Variables|Default|GetColorKeyIndex)) (>= (Variables|Default|GetColorKeyIndex) (Utilities|Array|Length (Variables|Default|GetKeys)))) ; If true, re-shuffle all keys and colors and reset colorkeyindex. Else, change next key's color
    ;[0.6013 0.7789 1] Shuffle and reset
    (Utilities|Array|Shuffle (Variables|Default|GetColor))
    (Utilities|Array|Shuffle (Variables|Default|GetKeys))
    (Variables|Default|SetColorKeyIndex 0))
  (Utilities|IsValid (Utilities|Array|Get(acopy) (Variables|Default|GetKeys) (Variables|Default|GetColorKeyIndex)) ; Does the key still exist?
    (:Is%20Valid
      (bind _returnvalue (Rendering|Material|CreateDynamicMaterialInstance (Variables|/Game/Blueprints/bp_key.bp_key_C|GetCylinder (Utilities|Array|Get(acopy) (Variables|Default|GetKeys) (Variables|Default|GetColorKeyIndex))) 0 "/Game/Materials/M_base.M_base" "None" :!class /Script/Engine.PrimitiveComponent))
      (Rendering|Material|SetVectorParameterValue _returnvalue "Base Color" (Math|Conversions|ToLinearColor(Color) (Utilities|Array|Get(acopy) (Variables|Default|GetColor) (Variables|Default|GetColorKeyIndex))) :!class /Script/Engine.MaterialInstanceDynamic))
    (:Is%20Not%20Valid
      ;[1 1 1] Reseet key array if one is missing
      (bind _outactors (Actor|GetAllActorsOfClass "/Game/Blueprints/bp_key.bp_key_C"))
      (Variables|Default|SetKeys _outactors)))
  (Math|Integer|IncrementInt (Variables|Default|GetColorKeyIndex)
    (:%20%20
      (Utilities|FlowControl|Delay 0.5)
      (CallFunction|ChangeKeyColor))))

(event EventBeginPlay
  (Utilities|FlowControl|Sequence
    (:then_0
      ;[1 1 1] Loop setup
      (CallFunction|SimpleGameLoop)
      (Input|EnableInput (Game|GetPlayerController 0))
      (CallFunction|RecursivveLoop))
    (:then_1
      ;[0.6589 0.4942 0.3187] Setup for lists
      (bind _outactors (Actor|GetAllActorsOfClass "/Game/Blueprints/bp_key.bp_key_C"))
      (Variables|Default|SetKeys _outactors)
      (CallFunction|ChangeKeyColor))))

(event Collision|EventActorBeginOverlap
  (params (OtherActor :type Actor%20Object%20Reference)))

(event EventTick
  (params (DeltaSeconds :type Float%20%28single-precision%29)))

(event Input|ActionEvents|InputActionStartWhileLoop
  (params (Key :type Key%20Structure :default "None"))
  (:Pressed
    (while (< (Variables|Default|GetwhileLoopCounter) 0)
      ;[1 1 1] body
      (Math|Integer|IncrementInt (Variables|Default|GetwhileLoopCounter)
        (:%20%20
          (Development|PrintString (Utilities|String|Append "This while loop has run " (Utilities|String|ToString(Integer) (Variables|Default|GetwhileLoopCounter)) " times.") true true (Math|Color|MakeColor (Math|Random|RandomFloat) (Math|Random|RandomFloat) (Math|Random|RandomFloat))))))
    (Development|PrintString "The while loop is done!")
    (Variables|Default|SetwhileLoopCounter 0)))

(event Input|KeyboardEvents|6
  (params (Key :type Key%20Structure :default "None"))
  (:Pressed
    (CallFunction|FirstArrayTest)))

(event Input|KeyboardEvents|5
  (params (Key :type Key%20Structure :default "None"))
  (:Pressed
    (CallFunction|ListAllNames)))

(fn ConstructionScript)