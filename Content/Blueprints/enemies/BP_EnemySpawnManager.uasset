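; Enemy spawn manager that runs endless waves, spawning one enemy at each BP_EnemySpawner in the level.
; On BeginPlay it caches every spawner, then spawns the first wave at their transforms, giving each enemy a reference back to itself and counting living enemies.
; The Re-Spawner event decrements that count and, once none remain, announces a new wave and spawns it after a short delay.
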(event Custom|Spawn%20Enemies
  (for _array_element (Variables|Default|GetSpawners)
    (bind _returnvalue (Game|SpawnActorfromClass "/Game/Blueprints/enemies/BP_Enemy.BP_Enemy_C" (Math|Transform|MakeTransform (.location (Transformation|GetWorldTransform (Variables|/Game/Blueprints/enemies/BP_EnemySpawner.BP_EnemySpawner_C|GetDefaultSceneRoot _array_element))) (.rotation (Transformation|GetWorldTransform (Variables|/Game/Blueprints/enemies/BP_EnemySpawner.BP_EnemySpawner_C|GetDefaultSceneRoot _array_element))) "1.000000,1.000000,1.000000") "Undefined" "MultiplyWithRoot" 0 0))
    (Variables|/Game/Blueprints/enemies/BP_Enemy.BP_Enemy_C|SetManager _returnvalue self)
    (Math|Integer|IncrementInt (Variables|Default|GetLivingEnemies))))

(event Custom|Re-Spawner
  (Math|Integer|DecrementInt (Variables|Default|GetLivingEnemies)
    (:%20%20
      (if (not (> (Variables|Default|GetLivingEnemies) 0))
        (Development|PrintString "New Wave Summoned!" true true "(R=1.000000,G=0.000000,B=0.215297,A=1.000000)" 5.0)
        (Utilities|FlowControl|Delay 5.0)
        (CallFunction|SpawnEnemies)))))

(event EventBeginPlay
  (Development|PrintString "Enemy Spawn Manager Is Ready" true true "(R=0.000000,G=0.906250,B=0.477972,A=1.000000)")
  (bind _outactors (Actor|GetAllActorsOfClass "/Game/Blueprints/enemies/BP_EnemySpawner.BP_EnemySpawner_C"))
  (Variables|Default|SetSpawners _outactors)
  (CallFunction|SpawnEnemies))

(fn ConstructionScript)